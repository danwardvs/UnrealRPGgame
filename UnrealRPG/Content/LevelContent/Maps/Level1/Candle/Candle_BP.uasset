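; Candle actor for Level1 that fakes a flickering flame with a point light animated every Tick.
; The light jumps to a random relative position within a cube bounded by LightRadiusMax.
; Intensity drifts by a random walk held between IntensityMin and IntensityMax.
; A clamped random walk on the green channel shifts the orange hue, with all changes applied per frame without delta-time scaling.
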(event `self.ReceiveBeginPlay`)

(event `self.ReceiveActorBeginOverlap`
  (params (OtherActor :type "Actor Object Reference")))

(event `self.ReceiveTick`
  (params (DeltaSeconds :type "Float (single-precision)"))
  (bind (_r _g _b) (`KismetMathLibrary.BreakColor` (struct :`R` 0.965 :`G` 0.481313 :`B` 0.14879 :`A` 1.0)))
  (bind _returnvalue (`KismetMathLibrary.RandomFloatInRange` (* (`self.LightRadiusMax`) -1.0) (`self.LightRadiusMax`)))
  (`SceneComponent.K2_SetRelativeLocation` (`self.PointLight`) (`KismetMathLibrary.MakeVector` _returnvalue _returnvalue _returnvalue) false false)
  (set `self.Intensity` (+ (`KismetMathLibrary.RandomFloatInRange` -100.0 100.0) (`self.Intensity`)))
  (if (> (`self.Intensity`) (`self.IntensityMax`))
    (set `self.Intensity` (`self.IntensityMax`))
    (elif (< (`self.Intensity`) (`self.IntensityMin`))
      (set `self.Intensity` (`self.IntensityMin`))))
  (`LightComponent.SetIntensity` (`self.PointLight`) (`self.Intensity`))
  (set `self.Color` (`KismetMathLibrary.FClamp` (+ (`self.Color`) (`KismetMathLibrary.RandomFloatInRange` -0.05 0.05)) 0.3 0.7))
  (`LightComponent.SetLightColor` (`self.PointLight`) (`KismetMathLibrary.MakeColor` _r (`self.Color`) _b) true))

(fn `UserConstructionScript`)